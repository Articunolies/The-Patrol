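; BP_LockerHide is a locker the player can hide in by pressing Hide within its trigger box.
; Box overlap enables or disables the locker's input and opens or closes a Gate guarding the key.
; Each press plays a door-swing timeline and toggles player visibility, collision and camera, blending the view between locker and player.
; A short delay then re-enables input and reopens the gate, allowing exit while player collision is off.
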(event OnComponentBeginOverlap(Box)
  (params (OverlappedComponent :type Primitive%20Component%20Object%20Reference) (OtherActor :type Actor%20Object%20Reference) (OtherComp :type Primitive%20Component%20Object%20Reference) (OtherBodyIndex :type Integer) (bFromSweep :type Boolean) (SweepResult :type Hit%20Result%20Structure%20%28by%20ref%29))
  (bind _asbp_player (Utilities|Casting|CastToBP_Player OtherActor))
  (Variables|Default|SetAs%20BP%20Player _asbp_player)
  (Input|EnableInput (Game|GetPlayerController 0))
  (Utilities|FlowControl|Gate true) ; enters at Open
)

(event OnComponentEndOverlap(Box)
  (params (OverlappedComponent :type Primitive%20Component%20Object%20Reference) (OtherActor :type Actor%20Object%20Reference) (OtherComp :type Primitive%20Component%20Object%20Reference) (OtherBodyIndex :type Integer))
  (bind _returnvalue (Game|GetPlayerController 0))
  (Utilities|Casting|CastToBP_Player OtherActor)
  (Input|DisableInput _returnvalue)
  (Utilities|FlowControl|Gate true) ; enters at Close
)

(event Input|ActionEvents|InputActionHide
  (params (Key :type Key%20Structure :default "None"))
  (:Pressed
    (Utilities|FlowControl|Gate true :!label _label
      (:Exit
        (Utilities|FlowControl|Sequence
          (:then_0
            (CallFunction|ToggleHide)
            (Utilities|FlowControl|Delay 0.2)
            (Input|EnableInput (Game|GetPlayerController 0))
            (goto _label Open))
          (:then_1
            (bind _doortrack (Timeline|OpenCloseDoorT PlayFromStart)
              (:Update
                (Transformation|SetRelativeRotation (Variables|Default|GetLocker_Door) (Math|Rotator|MakeRotator 0.0 0.0 (Math|Float|Lerp (Variables|Default|GetClosedAngle) (Variables|Default|GetOpen%20Angle) _doortrack)) false false)))))))))

(fn ConstructionScript)

(fn ToggleHide
  (bind _returnvalue (Game|GetPlayerController 0))
  (bind _as_bp_player (Variables|Default|GetAs%20BP%20Player))
  (if (Variables|Default|GetIsHiding)
    (Variables|Default|SetIsHiding false)
    (Development|PrintString "false")
    (Rendering|SetActorHiddenInGame _as_bp_player false)
    (Collision|SetActorEnableCollision _as_bp_player true)
    (Game|Player|SetViewTargetwithBlend _returnvalue _as_bp_player 0.6 "VTBlend_Linear" 0.0 false)
    (else
      (Variables|Default|SetIsHiding true)
      (Development|PrintString "true")
      (Rendering|SetActorHiddenInGame _as_bp_player true)
      (Collision|SetActorEnableCollision _as_bp_player false)
      (Game|Player|SetViewTargetwithBlend _returnvalue self 0.6 "VTBlend_Linear" 0.0 false))))