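; BP_RoamEnemy is a roaming enemy character that patrols, chases and ends the player's run when it attacks.
; Its Attack event opens the death UI level directly, then calls the OnAttackEnd dispatcher.
; It exposes its patrol route and maps a speed state from idle to sprinting onto the character's max walk speed.
; An explosion emitter on the capsule is present but never runs.
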(event Custom|Attack
  (Game|OpenLevel(byName) "DeathUILevel")
  (Default|CallOnAttackEnd))

(fn ConstructionScript)

(fn GetPatrolRoute
  (return (Variables|Default|GetPatrolRoute)))

(fn SetMovementSpeed
  (params (Speed :type E_EnemyMoveSpeed%20Enum :default "NewEnumerator4"))
  (bind _output_get (Variables|/Script/Engine.CharacterMovementComponent|SetMaxWalkSpeed (Variables|Character|GetCharacterMovement) (Utilities|Select :Index Speed :NewEnumerator4 0.0 :NewEnumerator0 1e+02 :NewEnumerator1 3e+02 :NewEnumerator5 1.2e+03)))
  (return _output_get))